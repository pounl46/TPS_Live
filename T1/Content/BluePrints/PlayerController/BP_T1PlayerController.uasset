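; Player controller that lets the player switch control between the BP_T1Character actors in the level.
; BeginPlay caches all of those actors in the T1Characters array.
; Pressing the 1 key increments NowIndex and wraps it by the array length with modulo, then PossessT1Character validates the index, unpossesses the current pawn and possesses the selected character.
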(event `self.ReceiveBeginPlay`
  (bind _outactors (`GameplayStatics.GetAllActorsOfClass` "/Game/BluePrints/Character/BP_T1Character.BP_T1Character_C"))
  (set `self.T1Characters` _outactors))

(event `Key|One`
  (params (Key :type "Key Structure"))
  (:`Pressed`
    (bind _result (`/Engine/EditorBlueprintResources/StandardMacros.IncrementInt` (`self.NowIndex`))
      (:`  `
        (`self.PossessT1Character` (mod _result (`KismetArrayLibrary.Array_Length` (`self.T1Characters`))))))))

(fn `PossessT1Character`
  (params (NewIndex :type Integer))
  (bind _t1characters (`self.T1Characters`))
  (if (`KismetArrayLibrary.Array_IsValidIndex` _t1characters NewIndex)
    (`self.UnPossess`)
    (`self.Possess` (`|GetArrayItem` _t1characters NewIndex))))

(fn `UserConstructionScript`)